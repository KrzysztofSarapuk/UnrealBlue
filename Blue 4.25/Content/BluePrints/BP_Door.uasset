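; BP_Door is a door that swings open when a ThirdPersonCharacter enters its Box and closes when the character leaves.
; The Doors timeline plays or reverses on overlap, scaling Angle to set the yaw of SMDoor.
; The swing sign comes from comparing the door's forward vector with the normalized direction to the character using a 1.0 tolerance, so it depends on the approach side.
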(event `self.Box.OnComponentBeginOverlap`
  (params (OverlappedComponent :type "PrimitiveComponent Object Reference") (OtherActor :type "Actor Object Reference") (OtherComp :type "PrimitiveComponent Object Reference") (OtherBodyIndex :type Integer) (bFromSweep :type Boolean) (SweepResult :type "HitResult Structure (by ref)"))
  (bind _asthird_person_character (cast `/Game/ThirdPersonBP/Blueprints/ThirdPersonCharacter` OtherActor))
  (set `self.direction` (== (`self.GetActorForwardVector`) (`KismetMathLibrary.Normal` (- (`self.K2_GetActorLocation` _asthird_person_character) (`self.K2_GetActorLocation`))) :`ErrorTolerance` 1.0))
  (bind (_direction _newtrack_0) (`Timeline|doors` :!label _label)
    (:`Update`
      (`SceneComponent.K2_SetRelativeRotation` (`self.SM_Door`) (`KismetMathLibrary.MakeRotator` 0.0 0.0 (* _newtrack_0 (`self.angle`) (`KismetMathLibrary.SelectFloat` -1.0 1.0 (`self.direction`)))) false false))))

(event `self.Box.OnComponentEndOverlap`
  (params (OverlappedComponent :type "PrimitiveComponent Object Reference") (OtherActor :type "Actor Object Reference") (OtherComp :type "PrimitiveComponent Object Reference") (OtherBodyIndex :type Integer))
  (cast `/Game/ThirdPersonBP/Blueprints/ThirdPersonCharacter` OtherActor)
  (goto _label :!via `Reverse`))

(fn `UserConstructionScript`)